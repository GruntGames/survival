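; KG_HealthPickUp is a pickup actor that restores health to an overlapping KG_CharacterBase.
; On overlap it adds HealthOffering to the character's Health, capped at the Health default of that character's class, then destroys itself.
; The class default serves as maximum health, and the pickup stays in place when Health already equals it.
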(event `self.ReceiveActorBeginOverlap`
  (params (OtherActor :type "Actor Object Reference"))
  (bind _askg_character_base (cast `/Game/BluePrints/KG_CharacterBase` OtherActor))
  (bind _health (defaults `/Game/BluePrints/KG_HealthPickUp` (`GameplayStatics.GetObjectClass` _askg_character_base)))
  (if (not (== _health (`/Game/BluePrints/KG_CharacterBase.health` _askg_character_base)))
    (set `/Game/BluePrints/KG_CharacterBase.health` (`KismetMathLibrary.FMin` _health (+ (`/Game/BluePrints/KG_CharacterBase.health` _askg_character_base) (`self.healthOffering`))) _askg_character_base)
    (`self.K2_DestroyActor`)))

(fn `UserConstructionScript`)