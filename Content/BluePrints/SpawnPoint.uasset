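; SpawnPoint is an actor that keeps one AI unit of a configurable class alive at its location.
; It spawns the unit on BeginPlay through SpawnAIFromClass and stores it in SpawnedUnit.
; Tick polls that reference and, once it is invalid, runs a RespawnTimer delay before calling the Respawn event to spawn a replacement.
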(event `Respawn`
  (bind _returnvalue (`AIBlueprintHelperLibrary.SpawnAIFromClass` (`self.class to spawn `) null (`self.K2_GetActorLocation`) :!label _label))
  (set `self.spawnedUnit` _returnvalue))

(event `self.ReceiveBeginPlay`
  (goto _label))

(event `self.ReceiveTick`
  (params (DeltaSeconds :type "Float (single-precision)"))
  (if (not (`KismetSystemLibrary.IsValid` (`self.spawnedUnit`)))
    (`KismetSystemLibrary.Delay` (`self.RespawnTimer`))
    (`self.Respawn`)))

(fn `UserConstructionScript`)