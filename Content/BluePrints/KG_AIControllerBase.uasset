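; Base AI controller that makes its pawn hunt and attack player-controlled characters, without a behavior tree.
; A looping timer runs ProcessAI, which sphere-overlaps pawns around the controller's location to acquire a player-controlled KG_CharacterBase as Target.
; A valid Target is kept and approached to the pawn's AttackRange, then focused and hit with UsePrimaryAttack.
; Without a target, the pawn wanders to random navigable points.
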(event `self.ReceiveBeginPlay`
  (`KismetSystemLibrary.K2_SetTimerDelegate` (delegate `ProcessAI`) 2.0 true))

(event `ProcessAI`
  (bind _returnvalue (`self.K2_GetPawn`))
  (`self.target`
    (:`then`
      (`|AIMoveTo` _returnvalue (0.0 0.0 0.0) (`self.target`) (`/Game/BluePrints/KG_CharacterBase.AttackRange` (cast `/Game/BluePrints/KG_CharacterBase` _returnvalue :!pure true)) :!label _label
        (:`OnSuccess`
          (bind _askg_character_base (cast `/Game/BluePrints/KG_CharacterBase` (`self.K2_GetPawn`)))
          (`self.K2_SetFocalPoint` (`self.K2_GetActorLocation` (`self.target`)))
          (`/Game/BluePrints/KG_CharacterBase.UsePrimary Attack` _askg_character_base))))
    (:`else`
      (bind _outactors (`KismetSystemLibrary.SphereOverlapActors_NEW` (`self.K2_GetActorLocation`) 1000.0 (`|MakeArray` "ObjectTypeQuery3" :!type "EObjectTypeQuery Enum") null (`|MakeArray` (`self.K2_GetPawn`) :!type "Actor Object Reference")))
      (for _array_element _outactors
        (bind _askg_character_base_2 (cast `/Game/BluePrints/KG_CharacterBase` _array_element))
        (if (`self.IsPlayerController` (`Pawn.GetController` _askg_character_base_2))
          (set `self.target` _askg_character_base_2)
          (break)))
      (`self.target`
        (:`then`
          (goto _label))
        (:`else`
          (`self.Wander`))))))

(event `Wander`
  (bind _returnvalue (`self.K2_GetPawn`))
  (`/Engine/EditorBlueprintResources/StandardMacros.IsValid` _returnvalue
    (:`Is Valid`
      (`|AIMoveTo` _returnvalue (`NavigationSystem.GetRandomPointInNavigableRadius` (`self.K2_GetActorLocation` _returnvalue) 2000.0)))))

(fn `UserConstructionScript`)