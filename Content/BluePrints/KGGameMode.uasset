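; KGGameMode is a game mode that runs wave-based enemy spawning.
; It loads each wave's class list into a shuffled queue, starting at BeginPlay, and a looping timer spawns one AI per tick at random PlayerStarts.
; CheckWaveComplete advances the wave once the queue and AI controllers are empty, but its OnDestroyed binding is disconnected, so waves never advance from this graph.
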(event `self.ReceiveBeginPlay`
  (`KismetSystemLibrary.K2_SetTimerDelegate` (delegate `SpawnEnemy`) 1.0 true)
  (`self.ResetGame`))

(event `SpawnEnemy`
  (if (> (`KismetArrayLibrary.Array_Length` (`self.current que`)) 0)
    (bind _outactors (`GameplayStatics.GetAllActorsOfClass` "/Script/Engine.PlayerStart"))
    (bind _item (`KismetArrayLibrary.Array_Get` _outactors (`KismetMathLibrary.RandomInteger` (`KismetArrayLibrary.Array_Length` _outactors))))
    (bind _returnvalue (`AIBlueprintHelperLibrary.SpawnAIFromClass` (`KismetArrayLibrary.Array_Get` (`self.current que`)) null (`self.K2_GetActorLocation` _item) (`self.K2_GetActorRotation` _item)))
    (`KismetArrayLibrary.Array_Remove` (`self.current que`))))

(event `CheckWave Complete` :!signature `self.OnDestroyed`
  (params (DestroyedActor :type "Actor Object Reference"))
  (if (== (`KismetArrayLibrary.Array_Length` (`self.current que`)) 0)
    (bind _outactors (`GameplayStatics.GetAllActorsOfClass` "/Game/BluePrints/KG_AIControllerBase.KG_AIControllerBase_C"))
    (if (== (`KismetArrayLibrary.Array_Length` _outactors) 0)
      (`self.StartNewWave`))))

(event `ResetGame`
  (bind _item_classtospawn (break `/Game/BluePrints/WaveStructs` (`KismetArrayLibrary.Array_Get` (`self.Waves`) (`self.WaveIndex`))))
  (set `self.WaveIndex` 0)
  (bind _output_get (set `self.current que` _item_classtospawn :!label _label))
  (`KismetArrayLibrary.Array_Shuffle` _output_get))

(event `StartNewWave`
  (`/Engine/EditorBlueprintResources/StandardMacros.IncrementInt` (`self.WaveIndex`)
    (:`  `
      (goto _label))))

(fn `UserConstructionScript`)