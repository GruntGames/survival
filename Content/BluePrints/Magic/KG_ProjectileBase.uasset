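; Base magic projectile Blueprint that damages characters it hits and bursts when destroyed.
; On overlap with any KG_CharacterBase other than its Instigator, it applies point-blank damage credited to the Instigator's controller, then destroys itself.
; The Destroyed event spawns an impulse particle effect and applies small-radius radial damage, so the burst follows any destruction and can add to the direct hit.
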(event `self.ReceiveActorBeginOverlap`
  (params (OtherActor :type "Actor Object Reference"))
  (bind _instigator (`self.Instigator`))
  (bind _askg_character_base (cast `/Game/BluePrints/KG_CharacterBase` OtherActor))
  (if (not (== _askg_character_base _instigator))
    (`GameplayStatics.ApplyDamage` _askg_character_base 50.0 (`Pawn.GetController` _instigator) self)
    (`self.K2_DestroyActor`)))

(event `self.ReceiveActorEndOverlap`
  (params (OtherActor :type "Actor Object Reference")))

(event `self.ReceiveDestroyed`
  (`GameplayStatics.SpawnEmitterAtLocation` "/Game/assets/effects/P_Impulse.P_Impulse" (`self.K2_GetActorLocation`))
  (`GameplayStatics.ApplyRadialDamage` :`BaseDamage` 50.0 :`Origin` (`self.K2_GetActorLocation`) :`DamageRadius` 20.0 :`DamageCauser` self :`InstigatedByController` (`Pawn.GetController` (`self.Instigator`))))

(fn `UserConstructionScript`)