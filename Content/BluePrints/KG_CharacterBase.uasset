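; Base knight character with sword melee, magic projectile attacks, health, flinching and death.
; BeginPlay attaches a spawned sword to the mesh socket; construction sets hair color and links the healthbar widget to the knight.
; Melee chains into a second montage section when re-triggered, and flinching blocks new attacks.
; Damage picks a flinch reaction from montage state, skipping it during listed attack moves; zero health plays death, then destroys sword and character.
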(event `self.ReceiveBeginPlay`
  (`self.Create Sword`))

(event `Melee_Atk`
  (bind _returnvalue (`SkeletalMeshComponent.GetAnimInstance` (`self.Mesh`)))
  (bind _returnvalue_2 (`AnimInstance.Montage_GetCurrentSection` _returnvalue "/Game/assets/Knight/Animations/KnightAttack_Montage.KnightAttack_Montage"))
  (if (`self.is Flinching`)
    _
    (elif (`AnimInstance.Montage_IsActive` _returnvalue "/Game/assets/Knight/Animations/KnightAttack_Montage.KnightAttack_Montage")
      (switch `name` _returnvalue_2
        (:`Attack 1`
          (`AnimInstance.Montage_SetNextSection` _returnvalue _returnvalue_2 "Attack 2" null)))
      (else
        (`self.PlayAnimMontage` "/Game/assets/Knight/Animations/KnightAttack_Montage.KnightAttack_Montage" 1.0 "Attack 1")))))

(event `Magic_Atk`
  (if (not (`self.is Flinching`))
    (`self.PlayAnimMontage` "/Game/assets/Knight/Animations/MagicShoot.MagicShoot")))

(event `LaunchMagicProjectile`
  (`|SpawnActorFromClass` "/Game/BluePrints/KG_ProjectileBase.KG_ProjectileBase_C" (`SceneComponent.K2_GetComponentToWorld` (`self.Arrow1`)) "Undefined" "OverrideRootScale" null self))

(event `Create Sword`
  (bind _returnvalue (`|SpawnActorFromClass` "/Game/BluePrints/BaseSword.BaseSword_C" (`self.GetTransform`) "Undefined" "OverrideRootScale"))
  (`self.K2_AttachToComponent` _returnvalue (`self.Mesh`) "sword" "SnapToTarget" "SnapToTarget" "SnapToTarget" false)
  (set `self.weapon` _returnvalue))

(event `UsePrimary Attack`
  (`self.Melee_Atk`))

(event `self.ReceiveAnyDamage`
  (params (Damage :type "Float (single-precision)") (DamageType :type "DamageType Object Reference") (InstigatedBy :type "Controller Object Reference") (DamageCauser :type "Actor Object Reference"))
  (bind _returnvalue (`SkeletalMeshComponent.GetAnimInstance` (`self.Mesh`)))
  (bind _output_get (set `self.health` (- (`self.health`) Damage)))
  (if (<= _output_get 0.0)
    (`/Engine/EditorBlueprintResources/StandardMacros.DoOnce` false
      (:`Completed`
        (set `self.is Flinching` false)
        (`CharacterMovementComponent.DisableMovement` (`self.CharacterMovement`))
        (bind _returnvalue_2 (`self.PlayAnimMontage` "/Game/assets/Knight/Animations/PlayerDeath.PlayerDeath"))
        (`KismetSystemLibrary.Delay` _returnvalue_2)
        (`self.K2_DestroyActor` (`self.weapon`))
        (`self.K2_DestroyActor`)))
    (else
      (set `self.is Flinching` true)
      (if (`AnimInstance.Montage_IsActive` _returnvalue "/Game/assets/Knight/Animations/KnightAttack_Montage.KnightAttack_Montage")
        (if (`KismetArrayLibrary.Array_Contains` (`self.AttackMoves`) (`AnimInstance.Montage_GetCurrentSection` _returnvalue "/Game/assets/Knight/Animations/KnightAttack_Montage.KnightAttack_Montage"))
          (set `self.is Flinching` false)
          (else
            (bind _returnvalue_3 (`self.PlayAnimMontage` null 1.0 "FlinchBig"))
            (`KismetSystemLibrary.Delay` _returnvalue_3)
            (set `self.is Flinching` false)))
        (else
          (bind _returnvalue_4 (`self.PlayAnimMontage` null 1.0 "FlinchSmall"))
          (`KismetSystemLibrary.Delay` _returnvalue_4)
          (set `self.is Flinching` false))))))

(fn `UserConstructionScript`
  (bind _returnvalue (`PrimitiveComponent.CreateDynamicMaterialInstance` (`self.Mesh`) 0 null))
  (`MaterialInstanceDynamic.SetVectorParameterValue` _returnvalue "hair color" (`self.hairColor`))
  (bind _asui_healthbar (cast `/Game/BluePrints/UI_Healthbar` (`WidgetComponent.GetUserWidgetObject` (`self.Healthbar`))))
  (`/Game/BluePrints/UI_Healthbar.Set Owning Knight` _asui_healthbar self))