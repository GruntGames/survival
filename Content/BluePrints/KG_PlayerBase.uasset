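; KG_PlayerBase is a player controller that drives a KG_CharacterBase pawn with cursor aiming, camera-relative movement and a pause menu.
; Each tick, a visibility trace under the visible cursor turns the living character's yaw toward the hit point.
; Movement axes push the pawn along the camera's up and right vectors, while actions trigger jump, melee and magic attacks.
; Escape or P shows a lazily created pause widget, switches to UI-only input and pauses the game.
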(event `self.ReceiveBeginPlay`
  (set `self.bShowMouseCursor` true))

(event `self.ReceiveTick`
  (params (DeltaSeconds :type "Float (single-precision)"))
  (`self.ProcessMouse`))

(event `ProcessMouse`
  (bind (_hitresult _returnvalue) (`self.GetHitResultUnderCursorByChannel` "TraceTypeQuery1"))
  (bind _returnvalue_2 (`self.K2_GetPawn`))
  (bind _returnvalue_3 (`self.K2_GetPawn`))
  (bind (_returnvalue_roll _returnvalue_pitch _returnvalue_yaw) (`KismetMathLibrary.BreakRotator` (`KismetMathLibrary.Conv_VectorToRotator` (`KismetMathLibrary.GetDirectionUnitVector` (`self.K2_GetActorLocation` _returnvalue_3) (`.Location` (`GameplayStatics.BreakHitResult` _hitresult))))))
  (`/Engine/EditorBlueprintResources/StandardMacros.IsValid` _returnvalue_2
    (:`Is Valid`
      (bind _askg_character_base (cast `/Game/BluePrints/KG_CharacterBase` _returnvalue_2))
      (if (and (> (`/Game/BluePrints/KG_CharacterBase.health` _askg_character_base) 0.0) _returnvalue)
        (`self.K2_SetActorRotation` _returnvalue_3 (`KismetMathLibrary.MakeRotator` 0.0 0.0 _returnvalue_yaw) false)))))

(event `InputAxis|up`
  (params (AxisValue :type "Float (single-precision)"))
  (bind _returnvalue (`self.K2_GetPawn`))
  (`/Engine/EditorBlueprintResources/StandardMacros.IsValid` _returnvalue
    (:`Is Valid`
      (`Pawn.AddMovementInput` _returnvalue (`SceneComponent.GetUpVector` (`PlayerCameraManager.TransformComponent` (`self.PlayerCameraManager`))) AxisValue false))))

(event `InputAxis|right`
  (params (AxisValue :type "Float (single-precision)"))
  (bind _returnvalue (`self.K2_GetPawn`))
  (`/Engine/EditorBlueprintResources/StandardMacros.IsValid` _returnvalue
    (:`Is Valid`
      (`Pawn.AddMovementInput` _returnvalue (`SceneComponent.GetRightVector` (`PlayerCameraManager.TransformComponent` (`self.PlayerCameraManager`))) AxisValue false))))

(event `InputAction|jump`
  (params (Key :type "Key Structure" :default "AnyKey"))
  (:`Pressed`
    (bind _ascharacter (cast `Character` (`self.K2_GetPawn`)))
    (`Character.Jump` _ascharacter)))

(event `InputAction|melee Attack`
  (params (Key :type "Key Structure" :default "AnyKey"))
  (:`Pressed`
    (bind _askg_character_base (cast `/Game/BluePrints/KG_CharacterBase` (`self.K2_GetPawn`)))
    (`/Game/BluePrints/KG_CharacterBase.Melee_Atk` _askg_character_base)))

(event `InputAction|Magic Attack`
  (params (Key :type "Key Structure" :default "AnyKey"))
  (:`Pressed`
    (bind _askg_character_base (cast `/Game/BluePrints/KG_CharacterBase` (`self.K2_GetPawn`)))
    (`/Game/BluePrints/KG_CharacterBase.Magic_Atk` _askg_character_base)))

(event `Key|Escape`
  (params (Key :type "Key Structure" :default "AnyKey"))
  (bind _pausemenuereference (`self.PauseMenueReference`))
  (:`Pressed`
    (`/Engine/EditorBlueprintResources/StandardMacros.IsValid` (`self.PauseMenueReference`) :!label _label
      (:`Is Valid`
        _)
      (:`Is Not Valid`
        (bind _returnvalue (`|CreateWidget` "/Game/Menus/PauseMenu/PauseMenuWidget.PauseMenuWidget_C"))
        (set `self.PauseMenueReference` _returnvalue)))
    (`WidgetBlueprintLibrary.SetInputMode_UIOnlyEx` (`GameplayStatics.GetPlayerController` 0) _pausemenuereference)
    (`UserWidget.AddToViewport` _pausemenuereference 0)
    (`GameplayStatics.SetGamePaused` true)))

(event `Key|P`
  (params (Key :type "Key Structure" :default "AnyKey"))
  (:`Pressed`
    (goto _label)))

(fn `UserConstructionScript`)